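; Spider character Blueprint that can attack, take damage, die and be knocked back.
; Attack raises an IsAttacking flag for a fixed delay, while AffectHealth applies a delta and, at zero, detaches the controller and destroys the actor after a pause.
; Impact stuns it by briefly simulating physics on the capsule with a launch velocity, then restores the saved rotation.
; The Explosion event is an empty stub.
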(event `/Game/iAttack.Attack`
  ;[1 1 1] Attack and wait for attack animation
  (set `self.isAttacking` true)
  (`KismetSystemLibrary.Delay` 1.0)
  (set `self.isAttacking` false))

(event `self.ReceiveBeginPlay`)

(event `/Game/OwnBPs/Blueprints/iDamageable.AffectHealth`
  (params (Delta :type "Float (single-precision)"))
  ;[1 1 1] Take damage and die
  (bind _output_get (set `self.Health` (+ Delta (`self.Health`))))
  (if (<= _output_get 0.0)
    (`self.DetachFromControllerPendingDestroy`)
    (`KismetSystemLibrary.Delay` 1.0)
    (`self.K2_DestroyActor`)))

(event `/Game/OwnBPs/Blueprints/iExplosion.Explosion`
  (params (Damage :type "Float (single-precision)"))
  ;[1 1 1] Get affected by explosion
)

(event `/Game/OwnBPs/Blueprints/iImpact.Impact`
  (params (XYForce :type "Float (single-precision)") (ZForce :type "Float (single-precision)") (ForceVector :type "Vector Structure") (StunTime :type "Float (single-precision)"))
  (bind _capsulecomponent (`self.CapsuleComponent`))
  ;[1 1 1] Knockback from Impact
  (set `self.isStunned` true)
  (`KismetSystemLibrary.PrintString` "Impact")
  (set `self.Rotation` (`SceneComponent.K2_GetComponentRotation` (`self.CapsuleComponent`)))
  (`PrimitiveComponent.SetSimulatePhysics` _capsulecomponent true)
  (`PrimitiveComponent.SetPhysicsLinearVelocity` _capsulecomponent (`KismetMathLibrary.MakeVector` (.x (* ForceVector XYForce)) (.y (* ForceVector XYForce)) ZForce) false "None")
  (`KismetSystemLibrary.Delay` StunTime)
  (`PrimitiveComponent.SetSimulatePhysics` _capsulecomponent false)
  (set `self.isStunned` false)
  (`SceneComponent.K2_SetWorldRotation` (`self.CapsuleComponent`) (`self.Rotation`) false false))

(fn `UserConstructionScript`
  (`PrimitiveComponent.CreateDynamicMaterialInstance` (`self.Mesh`) 0 "/Game/Characters/Materials/HeroTPP.HeroTPP"))