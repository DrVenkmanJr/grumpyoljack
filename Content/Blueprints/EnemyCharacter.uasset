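; Enemy character Blueprint that tracks health and removes itself from the game when it dies.
; AffectHealth adds a signed delta to Health, prints the result and destroys the actor at zero or below.
; The Explosion event is empty, and a disconnected chain that would briefly enable capsule physics simulation never runs.
; The construction script creates a dynamic material instance from HeroTPP on the mesh.
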(event `self.ReceiveBeginPlay`)

(event `/Game/OwnBPs/Blueprints/iDamageable.AffectHealth`
  (params (Delta :type "Float (single-precision)"))
  ;[1 1 1] Take damage and die
  (bind _output_get (set `self.Health` (+ Delta (`self.Health`))))
  (`KismetSystemLibrary.PrintString` (`KismetStringLibrary.Conv_DoubleToString` _output_get))
  (if (<= _output_get 0.0)
    (`self.K2_DestroyActor`)))

(event `/Game/OwnBPs/Blueprints/iExplosion.Explosion`
  (params (Damage :type "Float (single-precision)"))
  ;[1 1 1] Get affected by explosion
)

(fn `UserConstructionScript`
  (`PrimitiveComponent.CreateDynamicMaterialInstance` (`self.Mesh`) 0 "/Game/Characters/Materials/HeroTPP.HeroTPP"))