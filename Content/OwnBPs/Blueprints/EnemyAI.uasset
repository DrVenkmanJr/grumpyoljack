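; AI controller for spider enemies that chases the player and attacks on arrival.
; A looping timer started at BeginPlay repeatedly issues AIMoveTo toward the player while the controlled SpiderCharacter is neither stunned nor dead.
; A successful move sends an attack message to the pawn and passes a random amount from the damage range to the player through a health message.
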(event `self.ReceiveBeginPlay`
  (`KismetSystemLibrary.K2_SetTimer` null "TrackPlayer" 0.5 true))

(event `TrackPlayer`
  (bind _returnvalue (`self.K2_GetPawn`))
  (bind _returnvalue_2 (`GameplayStatics.GetPlayerCharacter` 0))
  (bind _asspider_character (cast `/Game/Blueprints/SpiderCharacter` _returnvalue))
  (if (`/Game/Blueprints/SpiderCharacter.isStunned` _asspider_character)
    _
    (elif (not (`/Game/Blueprints/SpiderCharacter.isDead` _asspider_character))
      (`|AIMoveTo` _returnvalue (0.0 0.0 0.0) _returnvalue_2
        (:`OnSuccess`
          (message `/Game/iAttack.Attack` _returnvalue)
          (bind _result (`/Engine/EditorBlueprintResources/StandardMacros.NegateFloat` (`KismetMathLibrary.RandomFloatInRange` (`self.MinDamage`) (`self.MaxDamage`)))
            (:`  `
              (message `/Game/OwnBPs/Blueprints/iDamageable.AffectHealth` _returnvalue_2 _result)
              (`KismetSystemLibrary.Delay` 0.1))))))))

(fn `UserConstructionScript`)