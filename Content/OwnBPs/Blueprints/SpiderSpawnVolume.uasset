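; Spawn volume actor that adds spider enemies to the level while keeping their count under a limit.
; Its SpawnSpider event counts every SpiderCharacter in the world and compares that to MaxNoEnemies.
; When below the cap, it spawns an AI spider at a random point inside the EnemySpawnBox bounds and prints a debug string.
; Nothing in this graph calls SpawnSpider, as BeginPlay, overlap and Tick are empty.
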(event `SpawnSpider`
  (bind _enemyspawnbox (`self.EnemySpawnBox`))
  (bind _outactors (`GameplayStatics.GetAllActorsOfClass` "/Game/Blueprints/SpiderCharacter.SpiderCharacter_C"))
  (if (< (`KismetArrayLibrary.Array_Length` _outactors) (`self.MaxNoEnemies`))
    (`KismetSystemLibrary.PrintString` "spawnspider")
    (`AIBlueprintHelperLibrary.SpawnAIFromClass` "/Game/Blueprints/SpiderCharacter.SpiderCharacter_C" null (`KismetMathLibrary.RandomPointInBoundingBox` (`SceneComponent.K2_GetComponentLocation` _enemyspawnbox) (`BoxComponent.GetScaledBoxExtent` _enemyspawnbox)))))

(fn `UserConstructionScript`)