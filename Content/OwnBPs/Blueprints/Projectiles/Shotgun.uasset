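; Shotgun Blueprint that fires a burst of pellets when its FireShotgun event is called.
; The event loops to spawn ShotgunPellet actors at the Arrow component's world location, adjusting for collisions but always spawning.
; Each pellet keeps the arrow's roll and gets random pitch and yaw offsets that are only positive, so the spread is skewed to one side of the aim rather than centered.
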(event `self.ReceiveBeginPlay`)

(event `FireShotgun`
  (for _ (range 10)
    (`|SpawnActorFromClass` "/Game/OwnBPs/Blueprints/Projectiles/ShotgunPellet.ShotgunPellet_C" (`KismetMathLibrary.MakeTransform` (.location (`SceneComponent.K2_GetComponentToWorld` (`self.Arrow`))) (`KismetMathLibrary.MakeRotator` (.roll (.rotation (`SceneComponent.K2_GetComponentToWorld` (`self.Arrow`)))) (+ (.pitch (.rotation (`SceneComponent.K2_GetComponentToWorld` (`self.Arrow`)))) (`KismetMathLibrary.RandomFloatInRange` 0.0 10.0)) (+ (.yaw (.rotation (`SceneComponent.K2_GetComponentToWorld` (`self.Arrow`)))) (`KismetMathLibrary.RandomFloatInRange` 0.0 10.0)))) "AdjustIfPossibleButAlwaysSpawn" "OverrideRootScale")))

(fn `UserConstructionScript`)