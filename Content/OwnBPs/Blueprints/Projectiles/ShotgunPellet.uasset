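; Shotgun pellet projectile that reacts to overlaps with tagged actors.
; On an "Enemy" overlap it sends health and impact messages carrying damage and knockback force, aimed along the player controller's forward vector rather than the pellet's.
; Enemy and "Environment" hits each spawn their own impact particle at the pellet and then destroy it, while other overlaps are ignored.
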(event `self.ReceiveBeginPlay`)

(event `self.ReceiveActorBeginOverlap`
  (params (OtherActor :type "Actor Object Reference"))
  (bind _returnvalue (`SceneComponent.K2_GetComponentLocation` (`self.pellet`)))
  (if (`self.ActorHasTag` OtherActor "Enemy")
    (message `/Game/OwnBPs/Blueprints/iDamageable.AffectHealth` OtherActor (`self.Damage`))
    (message `/Game/OwnBPs/Blueprints/iImpact.Impact` OtherActor (`self.XYForce`) (`self.ZForce`) (`self.GetActorForwardVector` (`GameplayStatics.GetPlayerController` 0)) 0.0)
    (`GameplayStatics.SpawnEmitterAtLocation` "/Game/Effects/ParticleSystems/Gameplay/Player/P_body_bullet_impact.P_body_bullet_impact" _returnvalue)
    (`self.K2_DestroyActor` :!label _label)
    (elif (`self.ActorHasTag` OtherActor "Environment")
      (`GameplayStatics.SpawnEmitterAtLocation` "/Game/StarterContent/Particles/P_Impact_Dust.P_Impact_Dust" _returnvalue)
      (goto _label))))

(fn `UserConstructionScript`)