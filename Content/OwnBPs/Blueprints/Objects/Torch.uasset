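; Torch actor that tracks its burn time and goes out by destroying its fire and light components once MaxBurnTime passes.
; The construction script attaches Burner to Shaft and TorchLight to Burner, while Tick accumulates Burntime.
; BeginPlay holds a delay-based flicker loop that alternately raises and lowers light intensity at random rates and durations.
; That loop only starts if Burntime already exceeds 90% of MaxBurnTime at BeginPlay.
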(event `self.ReceiveBeginPlay`
  (bind _isincreasing (`self.isIncreasing`))
  (bind _startintensity (`self.StartIntensity`))
  (bind _changerate (`self.ChangeRate`))
  (bind _currentintensity (`self.CurrentIntensity`))
  (bind _torchlight (`self.TorchLight`))
  (`LightComponent.SetIntensity` (`self.TorchLight`) _startintensity)
  (set `self.CurrentIntensity` _startintensity)
  (while (> (stale `self.ReceiveTick` _output_get) (* 0.9 (`self.MaxBurnTime`)))
    (set `self.ChangeRate` (`KismetMathLibrary.RandomFloatInRange` 0.01 0.05))
    (bind _output_get (set `self.ChangeTime` (`KismetMathLibrary.RandomFloatInRange` 0.1 2.0)))
    (while (<= (`self.Counter`) _output_get)
      (if _isincreasing
        (bind _output_get_2 (set `self.CurrentIntensity` (* (+ _changerate 1.0) _currentintensity)))
        (`LightComponent.SetIntensity` _torchlight _output_get_2)
        (else
          (bind _output_get_3 (set `self.CurrentIntensity` (* (- 1.0 _changerate) _currentintensity)))
          (`LightComponent.SetIntensity` _torchlight _output_get_3)))
      (`KismetSystemLibrary.Delay` 0.1)
      (set `self.Counter` (+ 0.1 (`self.Counter`)))
      (`KismetSystemLibrary.PrintString` (`KismetStringLibrary.Conv_DoubleToString` (`self.CurrentIntensity`))))
    (set `self.isIncreasing` (not _isincreasing))
    (set `self.Counter` 0.0))
  (while false
    _))

(event `self.ReceiveTick`
  (params (DeltaSeconds :type "Float (single-precision)"))
  (bind _output_get (set `self.Burntime` (+ DeltaSeconds (`self.Burntime`))))
  (if (> _output_get (`self.MaxBurnTime`))
    (`ActorComponent.K2_DestroyComponent` (`self.TorchFire`))
    (`ActorComponent.K2_DestroyComponent` (`self.TorchLight`))))

(fn `UserConstructionScript`
  (bind _burner (`self.Burner`))
  (bind _torchlight (`self.TorchLight`))
  (`SceneComponent.K2_AttachToComponent` _burner (`self.Shaft`) "None" "KeepRelative" "KeepRelative" "KeepRelative" true)
  (`SceneComponent.K2_AttachToComponent` _torchlight _burner "None" "KeepRelative" "KeepRelative" "KeepRelative" true)
  (`SceneComponent.K2_AttachToComponent` _torchlight _burner "None" "KeepRelative" "KeepRelative" "KeepRelative" true))