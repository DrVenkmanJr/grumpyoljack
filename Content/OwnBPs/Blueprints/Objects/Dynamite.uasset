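; Throwable dynamite actor that explodes after a burning fuse runs down, knocking back and damaging nearby pawns.
; ThrowDynamite enables physics, shows the burn effect and sinks the fuse over FuseLength, then triggers the explosion and radial impulse.
; Pawns within DamageRadius with unobstructed line of sight receive distance-scaled knockback with stun, plus damage, through messages.
; It then plays a sound, removes the visible parts and destroys itself after a short delay.
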(event `ThrowDynamite`
  (bind _returnvalue (`self.K2_GetActorLocation`))
  (bind _damageradius (`self.DamageRadius`))
  (`SceneComponent.SetVisibility` (`self.BurningFuse`) true false)
  (`PrimitiveComponent.SetSimulatePhysics` (`self.Capsule`) true)
  (`KismetSystemLibrary.MoveComponentTo` (`self.Fuse`) (0.0 0.0 -5.0) (struct) false false (`self.FuseLength`))
  (`ActorComponent.Activate` (`self.Explosion`) false)
  (`RadialForceComponent.FireImpulse` (`self.RadialForce`))
  (bind _outactors (`GameplayStatics.GetAllActorsOfClass` "/Script/Engine.Pawn"))
  (for _array_element _outactors
    ;[1 1 1] Is Within Damage Radius?
    (set `self.CurrentTarget` _array_element)
    (bind _returnvalue_2 (`self.K2_GetActorLocation` _array_element))
    (bind (_outhit _returnvalue_3) (`KismetSystemLibrary.LineTraceSingle` _returnvalue _returnvalue_2 "TraceTypeQuery1" false _outactors))
    (bind _returnvalue_4 (- _returnvalue_2 _returnvalue))
    (bind _returnvalue_5 (`KismetMathLibrary.VSize` _returnvalue_4))
    (if (and (not _returnvalue_3) (< _returnvalue_5 _damageradius))
      (`KismetSystemLibrary.PrintString` "ExplosiveImpact")
      (bind _returnvalue_6 (`KismetMathLibrary.FMax` (* (/ _damageradius _returnvalue_5) (`self.Force`)) 100.0))
      (message `/Game/OwnBPs/Blueprints/iImpact.Impact` (`self.CurrentTarget`) _returnvalue_6 _returnvalue_6 (`KismetMathLibrary.Normal` (`KismetMathLibrary.MakeVector` (.x _returnvalue_4) (.y _returnvalue_4) (`KismetMathLibrary.Abs` (.z _returnvalue_4)))) (`self.StunTime`))
      (message `/Game/OwnBPs/Blueprints/iDamageable.AffectHealth` (`self.CurrentTarget`) -100.0)))
  (`GameplayStatics.PlaySoundAtLocation` "/Game/StarterContent/Audio/Explosion01.Explosion01")
  (`ActorComponent.K2_DestroyComponent` (`self.TNT`))
  (`ActorComponent.K2_DestroyComponent` (`self.Fuse`))
  (`ActorComponent.K2_DestroyComponent` (`self.BurningFuse`))
  (`KismetSystemLibrary.Delay` 2.0)
  (`self.K2_DestroyActor`))

(fn `UserConstructionScript`
  (`SceneComponent.SetVisibility` (`self.BurningFuse`) false false))